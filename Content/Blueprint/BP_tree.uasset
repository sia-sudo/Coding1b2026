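; BP_tree is a tree actor that enlarges its static mesh shortly after play begins.
; BeginPlay passes through a DoN node once, waits a random few seconds, then calls Grow, which adds a random amount to the mesh's relative scale.
; With no loop, growth happens only once.
; A follow-up branch to disable collision compares a random 3–5 value to zero, so it never runs.
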(event `self.ReceiveBeginPlay`
  (bind _returnvalue (`KismetMathLibrary.RandomFloatInRange` 3.0 5.0))
  (`/Engine/EditorBlueprintResources/StandardMacros.Do N` (`KismetMathLibrary.RandomIntegerInRange` 1 5)
    (:`Exit`
      (`KismetSystemLibrary.Delay` _returnvalue)
      (`self.grow`)
      (if (== _returnvalue 0.0)
        (`PrimitiveComponent.SetCollisionEnabled` (`self.SM_Generic_Tree_03`) "NoCollision")
        (`KismetSystemLibrary.PrintText` "collision enabled")))))

(event `grow`
  (bind _sm_generic_tree_03 (`self.SM_Generic_Tree_03`))
  (`SceneComponent.SetRelativeScale3D` _sm_generic_tree_03 (+ (`SceneComponent.RelativeScale3D` _sm_generic_tree_03) (`KismetMathLibrary.RandomFloatInRange` 0.2 0.4))))

(fn `UserConstructionScript`)