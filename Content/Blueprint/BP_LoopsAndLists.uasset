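; BP_LoopsAndLists is a demo actor for loop and array techniques, using printed text and BP_tree actors.
; BeginPlay starts an endless three-second Delay loop and a while countdown that prints in cycling colors.
; The Delay loop calls a timed loop over shuffled trees, whose rotation targets itself, with an index that never resets.
; An uncalled for-each event randomly yaws every tree at once.
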(event `self.ReceiveBeginPlay`
  (`KismetSystemLibrary.PrintText` "Loops and lists started")
  (`self.Simple loop`)
  (`self.WhileLoop Function`))

(event `Simple loop`
  (`KismetSystemLibrary.PrintText` "Inside simple loop waiting 3 seconds" :!label _label)
  (`self.Loop array overtime`)
  (`KismetSystemLibrary.Delay` 3.0)
  (goto _label))

(event `WhileLoop Function`
  (bind _colors (`self.Colors`))
  (while (> (`self.WhileCounter`) 0)
    (`KismetSystemLibrary.PrintText` (`|FormatText` "this is loount{count} Ran after {seconds}" (`self.WhileCounter`) (`KismetTextLibrary.Conv_DoubleToText` (`GameplayStatics.GetRealTimeSeconds`) "HalfToEven")) true true (`|GetArrayItem` _colors (mod (`self.WhileCounter`) (`KismetArrayLibrary.Array_Length` _colors))) 20.0)
    (`/Engine/EditorBlueprintResources/StandardMacros.DecrementInt` (`self.WhileCounter`)) ; decrement int
  ))

(event `Change Trees For Each`
  (bind _outactors (`GameplayStatics.GetAllActorsOfClass` "/Game/Blueprint/BP_tree.BP_tree_C"))
  (for _array_element _outactors
    (`self.K2_SetActorRelativeRotation` _array_element (`KismetMathLibrary.MakeRotator` 0.0 0.0 (`KismetMathLibrary.RandomFloatInRange` 0.0 360.0)) false false))
  (`KismetSystemLibrary.PrintText` "Trees have been rotated"))

(event `Loop array overtime`
  (bind _outactors (`GameplayStatics.GetAllActorsOfClass` "/Game/Blueprint/BP_tree.BP_tree_C"))
  (`KismetArrayLibrary.Array_Shuffle` _outactors)
  (if (< (`self.overtime index`) (`KismetArrayLibrary.Array_Length` _outactors)) :!label _label_2
    (`self.K2_SetActorRelativeRotation` (`KismetMathLibrary.MakeRotator` 0.0 0.0 (`KismetMathLibrary.RandomFloatInRange` 0.0 360.0)))
    (`/Engine/EditorBlueprintResources/StandardMacros.IncrementInt` (`self.overtime index`)
      (:`  `
        (`KismetSystemLibrary.Delay` 0.2)
        (goto _label_2)))))

(fn `UserConstructionScript`)