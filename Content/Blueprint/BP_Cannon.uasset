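; BP_Cannon is a cannon actor that fires BP_Cannonball projectiles automatically and continuously from the start of play.
; BeginPlay runs an endless Delay loop that calls the Fire event roughly ten times a second.
; Fire prints a debug message, spawns a cannonball at the Spawnpoint transform, and launches its SMChamferCube with a mass-independent AddForce along the Spawnpoint's forward vector.
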(event `self.ReceiveBeginPlay`
  (`KismetSystemLibrary.Delay` 0.1 :!label _label)
  (`self.Fire`)
  (goto _label))

(event `Fire`
  (`KismetSystemLibrary.PrintText` (`|FormatText` "Firing the {count}" _))
  (bind _returnvalue (`|SpawnActorFromClass` "/Game/Blueprint/BP_Cannonball.BP_Cannonball_C" (`SceneComponent.K2_GetComponentToWorld` (`self.Spawnpoint`)) "Undefined" "MultiplyWithRoot" null null))
  (`PrimitiveComponent.AddForce` (`/Game/Blueprint/BP_Cannonball.SM_ChamferCube` _returnvalue) (* (`SceneComponent.GetForwardVector` (`self.Spawnpoint`)) 100000.0) "None" true))

(fn `UserConstructionScript`)